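; BP_InfoText is an in-world display that shows the player's score and multiplier from BP_VRGameMode.
; On BeginPlay it finds and caches the game mode with GetActorOfClass.
; Each Tick it polls Point and Multiplier and writes them to two text render components, formatting the multiplier with an "x" prefix and limited decimals.
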(event `self.ReceiveBeginPlay`
  (bind _returnvalue (`GameplayStatics.GetActorOfClass` "/Game/SLICE/BP_VRGameMode.BP_VRGameMode_C"))
  (set `self.VRGameMode` _returnvalue))

(event `self.ReceiveTick`
  (params (DeltaSeconds :type "Float (single-precision)"))
  (bind _vrgamemode (`self.VRGameMode`))
  (`TextRenderComponent.K2_SetText` (`self.TextRender - ScoreValue`) (`KismetTextLibrary.Conv_IntToText` (`/Game/SLICE/BP_VRGameMode.Point` _vrgamemode)))
  (`TextRenderComponent.K2_SetText` (`self.TextRender - MultiplierValue`) (`KismetTextLibrary.Conv_StringToText` (`KismetStringLibrary.Concat_StrStr` "x" (`KismetTextLibrary.Conv_TextToString` (`KismetTextLibrary.Conv_DoubleToText` (`/Game/SLICE/BP_VRGameMode.Multiplier` _vrgamemode) "HalfToEven" false true 1 324 0 2))))))

(fn `UserConstructionScript`)