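; Spawn modifier for the slicing game that acts as a move speed malus on the sliceable object owning it.
; It overrides ApplySpawnEffect, calls the parent, then casts the owner to BP_Sliceable and scales its MoveSpeed by Multiplier.
; If the owner is not a BP_Sliceable, it prints an on-screen error naming that owner.
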(fn `ApplySpawnEffect`
  (bind _returnvalue (`self.GetOwner`))
  (`parent.ApplySpawnEffect`)
  (bind _asbp_sliceable (cast `/Game/SLICE/BP_Sliceable` _returnvalue)
    (:`then`
      (set `/Game/SLICE/BP_Sliceable.moveSpeed` (* (`/Game/SLICE/BP_Sliceable.moveSpeed` _asbp_sliceable) (`self.Multiplier`)) _asbp_sliceable))
    (:`CastFailed`
      (`KismetSystemLibrary.PrintString` (`KismetStringLibrary.Concat_StrStr` "Not a child of SliceableObject \nOwner is : " (`KismetSystemLibrary.GetDisplayName` _returnvalue)) true true (struct :`R` 1.0 :`B` 0.07426 :`A` 1.0) 22.0))))