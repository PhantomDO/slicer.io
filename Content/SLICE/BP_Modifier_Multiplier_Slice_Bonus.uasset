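; BP_Modifier_Multiplier_Slice_Bonus is a slice bonus modifier that boosts the game's multiplier when its slice effect is applied.
; ApplySliceEffect runs the parent effect, then calls BoostMultiplier on BP_VRGameMode with a random value drawn from the RangeMultiplier vector's X and Y bounds.
; The boost is skipped if the game mode cast fails, and BeginPlay only forwards to the parent.
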(event `self.ReceiveBeginPlay`
  (`parent.ReceiveBeginPlay`))

(fn `ApplySliceEffect`
  (bind (_x _y) (`KismetMathLibrary.BreakVector2D` (`self.RangeMultiplier`)))
  (`parent.ApplySliceEffect`)
  (bind _asbp_vrgame_mode (cast `/Game/SLICE/BP_VRGameMode` (`GameplayStatics.GetGameMode`)))
  (`/Game/SLICE/BP_VRGameMode.Boost Multiplier` _asbp_vrgame_mode (`KismetMathLibrary.RandomFloatInRange` _x _y)))