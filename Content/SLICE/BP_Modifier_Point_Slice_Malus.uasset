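; Sliceable point modifier for a VR game that penalizes the player when sliced and awards bonus points through its unslice effect.
; It extends a parent Blueprint by overriding the slice and unslice effect functions, calling the parent logic first.
; Each override casts the game mode to BP_VRGameMode, passing MalusPoint to ApplyMalusPoint on slice and BonusPoint to ApplyBonusPoint on unslice.
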(event `self.ReceiveBeginPlay`
  (`parent.ReceiveBeginPlay`))

(fn `ApplySliceEffect`
  (`parent.ApplySliceEffect`)
  (bind _asbp_vrgame_mode (cast `/Game/SLICE/BP_VRGameMode` (`GameplayStatics.GetGameMode`)))
  (`/Game/SLICE/BP_VRGameMode.ApplyMalusPoint` _asbp_vrgame_mode (`self.MalusPoint`)))

(fn `ApplyUnsliceEffect`
  (`parent.ApplyUnsliceEffect`)
  (bind _asbp_vrgame_mode (cast `/Game/SLICE/BP_VRGameMode` (`GameplayStatics.GetGameMode`)))
  (`/Game/SLICE/BP_VRGameMode.ApplyBonusPoint` _asbp_vrgame_mode (`self.BonusPoint`)))