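; BP_Sliceable is an actor that flies in a straight line toward the player's position at spawn and can be sliced.
; BeginPlay copies its static mesh into a hidden procedural mesh with convex collision.
; Slice cuts that mesh into two capped physics halves, reveals it, pushes the halves apart, fires each Modifier's slice effect and sets a short lifespan.
; Tick moves the actor, triggering unslice effects and destroying it once it passes the player.
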(event `self.ReceiveBeginPlay`
  (`SceneComponent.SetVisibility` (`self.ProceduralMesh`) false false)
  (`SceneComponent.SetVisibility` (`self.Mesh`) true false)
  (`KismetProceduralMeshLibrary.CopyProceduralMeshFromStaticMeshComponent` (`self.Mesh`) 0 (`self.ProceduralMesh`))
  (bind _vertices (`KismetProceduralMeshLibrary.GetSectionFromStaticMesh` (`StaticMeshComponent.StaticMesh` (`self.Mesh`))))
  (`ProceduralMeshComponent.AddCollisionConvexMesh` (`self.ProceduralMesh`) _vertices)
  (bind _returnvalue (`self.GetDirectionToPlayer`))
  (set `self._directionToFollow` _returnvalue)
  (bind _rotation (`self.GetRotationToPlayer`))
  (`self.K2_SetActorRotation` _rotation)
  (`SceneComponent.K2_SetWorldRotation` (`self.ProceduralMesh`) _rotation false false))

(event `self.ReceiveTick`
  (params (DeltaSeconds :type "Float (single-precision)"))
  (`self.MoveToPlayer` DeltaSeconds)
  (bind _returnvalue (`self.IsBehindPlayer`))
  (if _returnvalue
    (for _array_element (`self.modifiers`)
      (if (`KismetSystemLibrary.IsValid` _array_element)
        (`/Game/SLICE/BP_Modifier.ApplyUnsliceEffect` _array_element)
        (else
          (`KismetSystemLibrary.PrintString` (`KismetStringLibrary.Concat_StrStr` "Actor Component not valid : " (`KismetSystemLibrary.GetDisplayName` _array_element)) true true (struct :`G` 0.66 :`B` 1.0 :`A` 1.0) 12.0))))
    (`self.K2_DestroyActor`)))

(fn `GetDirectionToPlayer`
  (returns (ReturnValue :type "Vector Structure"))
  (bind (_returnvalue_x _returnvalue_y) (`KismetMathLibrary.BreakVector` (`self.K2_GetActorLocation`)))
  (bind (_returnvalue_x_2 _returnvalue_y_2) (`KismetMathLibrary.BreakVector` (`self.K2_GetActorLocation` (`GameplayStatics.GetPlayerController` 0))))
  (return (`KismetMathLibrary.Normal` (`KismetMathLibrary.MakeVector` (- _returnvalue_x_2 _returnvalue_x) (- _returnvalue_y_2 _returnvalue_y)))))

(fn `GetRotationToPlayer`
  (returns (Rotation :type "Rotator Structure"))
  (return (`KismetMathLibrary.FindLookAtRotation` (`self.K2_GetActorLocation`) (`self.K2_GetActorLocation` (`GameplayStatics.GetPlayerController` 0)))))

(fn `IsBehindPlayer`
  (returns (ReturnValue :type Boolean))
  (bind _returnvalue (`self.GetDirectionToPlayer`))
  (return (<= (`KismetMathLibrary.Dot_VectorVector` _returnvalue (`KismetMathLibrary.GetForwardVector` (`self.K2_GetActorRotation`))) 0.0)))

(fn `MoveToPlayer`
  (params (DeltaTime :type "Float (double-precision)"))
  (`self.K2_SetActorLocation` (+ (`self.K2_GetActorLocation`) (* (`self._directionToFollow`) (* (`self.moveSpeed`) DeltaTime)))))

(fn `Slice`
  (params (`Slicer Position` :type "Vector Structure") (`Slicer Normal` :type "Vector Structure") (ProcMesh :type "ProceduralMeshComponent Object Reference") (EnterPosition :type "Vector Structure"))
  (bind _outotherhalfprocmesh (`KismetProceduralMeshLibrary.SliceProceduralMesh` ProcMesh `Slicer Position` `Slicer Normal` true "CreateNewSectionForCap" (`PrimitiveComponent.GetMaterial` (`self.Mesh`) 0)))
  (`PrimitiveComponent.SetSimulatePhysics` _outotherhalfprocmesh true)
  (`PrimitiveComponent.SetSimulatePhysics` ProcMesh true)
  (`PrimitiveComponent.SetCollisionResponseToAllChannels` _outotherhalfprocmesh "ECR_Block")
  (`PrimitiveComponent.SetCollisionResponseToChannel` _outotherhalfprocmesh "ECC_PhysicsBody" "ECR_Overlap")
  (`PrimitiveComponent.AddRadialImpulse` _outotherhalfprocmesh EnterPosition 100.0 250.0 "RIF_Linear" true)
  (`PrimitiveComponent.AddRadialImpulse` ProcMesh EnterPosition 100.0 250.0 "RIF_Linear" true)
  (`SceneComponent.SetVisibility` (`self.Mesh`) false false)
  (`SceneComponent.SetVisibility` (`self.ProceduralMesh`) true false)
  (for _array_element (`self.modifiers`)
    (`/Game/SLICE/BP_Modifier.ApplySliceEffect` _array_element))
  (`self.SetLifeSpan` 5.0))

(fn `UserConstructionScript`)