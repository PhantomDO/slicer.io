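; Spawner actor for the slicing game that periodically spawns SpawnableObject at reduced scale, in one of three random height lanes around its own position.
; Tick polls CanSpawn against game time; FireRate is added both when storing NextFire and when testing it, so later spawns come two FireRate intervals apart.
; Each spawned BP_Sliceable receives unique modifiers from BP_VRGameMode and has its MoveSpeed scaled by the game mode's Multiplier.
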(event `self.ReceiveBeginPlay`
  (set `self._nextFire` 0.0))

(event `self.ReceiveTick`
  (params (DeltaSeconds :type "Float (single-precision)"))
  (bind (_returnvalue_location _returnvalue_rotation) (`KismetMathLibrary.BreakTransform` (`self.GetTransform`)))
  (bind (_canspawn _nextfire) (`self.CanSpawn`))
  (if _canspawn
    (set `self._nextFire` _nextfire)
    (bind _returnvalue (`|SpawnActorFromClass` (`self.SpawnableObject`) (`KismetMathLibrary.MakeTransform` (+ _returnvalue_location (`KismetMathLibrary.MakeVector` 0.0 0.0 (`KismetMathLibrary.Conv_IntToDouble` (* (`KismetMathLibrary.RandomIntegerInRange` -1 1) 40)))) _returnvalue_rotation (0.6 0.6 0.6)) "AlwaysSpawn" "OverrideRootScale" null null))
    (bind _asbp_sliceable (cast `/Game/SLICE/BP_Sliceable` _returnvalue))
    (bind _asbp_vrgame_mode (cast `/Game/SLICE/BP_VRGameMode` (`GameplayStatics.GetGameMode`)))
    (`/Game/SLICE/BP_VRGameMode.AddUniqueModifiers` _asbp_vrgame_mode _asbp_sliceable)
    (set `/Game/SLICE/BP_Sliceable.moveSpeed` (* (`/Game/SLICE/BP_Sliceable.moveSpeed` _asbp_sliceable) (`/Game/SLICE/BP_VRGameMode.Multiplier` _asbp_vrgame_mode)) _asbp_sliceable)))

(fn `CanSpawn`
  (returns (canSpawn :type Boolean) (nextFire :type "Float (double-precision)"))
  (bind _returnvalue (`GameplayStatics.GetTimeSeconds`))
  (bind _firerate (`self.FireRate`))
  (return (>= _returnvalue (+ (`self._nextFire`) _firerate)) (+ _returnvalue _firerate)))

(fn `UserConstructionScript`)