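; VR slicing game mode that tracks points and a multiplier and assigns random modifier components to sliceable objects.
; On BeginPlay it instantiates each modifier class on itself as a template for tag lookups.
; Bonuses are scaled by the multiplier, while maluses subtract points and reset it.
; AddUniqueModifiers draws distinct random modifiers per sliceable, using gameplay tags to prune opposing effects from the remaining pool after each pick.
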(event `self.ReceiveBeginPlay`
  (for _array_element (`self.Modifiers`)
    (bind _returnvalue (`|AddComponentByClass` _array_element))
    (`KismetArrayLibrary.Array_AddUnique` (`self.ModifierInstances`) _returnvalue)
    (set `self.Multiplier` 1.0)
    (set `self.Point` 0)))

(fn `AddUniqueModifiers`
  (params (Sliceable :type "/Game/SLICE/BP_Sliceable Object Reference"))
  (locals (Altered :type "GameplayTagContainer Structure") (Slice :type "GameplayTagContainer Structure") (RandomModifier :type "/Game/SLICE/BP_Modifier Object Reference"))
  (bind _modifierscopy (`self.ModifiersCopy`))
  (bind _output_get (set `self.ModifiersCopy` (`self.ModifierInstances`)))
  (for _ (range (+ (`KismetMathLibrary.RandomIntegerInRange` 1 (`self.MaxModifierOnSpawn`)) 1))
    (if (> (`KismetArrayLibrary.Array_Length` _output_get) 0)
      (`|ExecutionSequence`
        (:`then_0`
          (bind _output_get_2 (set `local.RandomModifier` (`KismetArrayLibrary.Array_Random` _output_get)))
          (`|SwitchGameplayTagContainer` (`/Game/SLICE/BP_Modifier.Altered Tag Container` _output_get_2)
            (:`(GameplayTags=((TagName="Altered.Multiplier")))`
              (bind _slice_tag_container (`/Game/SLICE/BP_Modifier.Slice Tag Container` _output_get_2))
              (`|SwitchGameplayTagContainer` _slice_tag_container
                (:`(GameplayTags=((TagName="Slice.Bonus")))`
                  (`self.RemoveAllOppositeTags` _modifierscopy (struct :`GameplayTags` (struct :`(TagName` "Unslice.Malus") :`(TagName` "Slice.Malus")))))
                (:`(GameplayTags=((TagName="Slice.Malus")))`
                  (`self.RemoveAllOppositeTags` _modifierscopy (struct :`GameplayTags` (struct :`(TagName` "Slice.Bonus") :`(TagName` "Unslice.Malus")))))
                (:`(GameplayTags=((TagName="Unslice.Bonus")))`
                  (`self.RemoveAllOppositeTags` _modifierscopy (struct :`GameplayTags` (struct :`(TagName` "Unslice.Malus") :`(TagName` "Slice.Bonus")))))
                (:`(GameplayTags=((TagName="Unslice.Malus")))`
                  (`self.RemoveAllOppositeTags` _modifierscopy (struct :`GameplayTags` (struct :`(TagName` "Unslice.Bonus") :`(TagName` "Slice.Malus")))))))
            (:`(GameplayTags=((TagName="Altered.Point")))`
              (`|SwitchGameplayTagContainer` _slice_tag_container
                (:`(GameplayTags=((TagName="Slice.Bonus")))`
                  (`self.RemoveAllOppositeTags` _modifierscopy (struct :`GameplayTags` (struct :`(TagName` "Unslice.Malus") :`(TagName` "Slice.Malus")))))
                (:`(GameplayTags=((TagName="Slice.Malus")))`
                  (`self.RemoveAllOppositeTags` _modifierscopy (struct :`GameplayTags` (struct :`(TagName` "Slice.Bonus") :`(TagName` "Unslice.Malus")))))
                (:`(GameplayTags=((TagName="Unslice.Bonus")))`
                  (`self.RemoveAllOppositeTags` _modifierscopy (struct :`GameplayTags` (struct :`(TagName` "Unslice.Malus") :`(TagName` "Slice.Bonus")))))
                (:`(GameplayTags=((TagName="Unslice.Malus")))`
                  (`self.RemoveAllOppositeTags` _modifierscopy (struct :`GameplayTags` (struct :`(TagName` "Unslice.Bonus") :`(TagName` "Slice.Malus")))))))
            (:`(GameplayTags=((TagName="Altered.Movespeed")))`
              (`|SwitchGameplayTagContainer` _slice_tag_container
                (:`(GameplayTags=((TagName="Spawn.Bonus")))`
                  (`self.RemoveAllOppositeTags` _modifierscopy (struct :`GameplayTags` (struct :`(TagName` "Spawn.Malus")))))
                (:`(GameplayTags=((TagName="Spawn.Malus")))`
                  (`self.RemoveAllOppositeTags` _modifierscopy (struct :`GameplayTags` (struct :`(TagName` "Spawn.Bonus")))))))))
        (:`then_1`
          (bind _returnvalue (`|AddComponentByClass` Sliceable (`|GetArrayItem` (`self.Modifiers`) (`KismetArrayLibrary.Array_Find` (`self.ModifierInstances`) (`local.RandomModifier`)))))
          (`KismetArrayLibrary.Array_AddUnique` (`/Game/SLICE/BP_Sliceable.modifiers` Sliceable) _returnvalue)
          (`KismetArrayLibrary.Array_RemoveItem` (`self.ModifiersCopy`) (`local.RandomModifier`))))
      (else
        (break))))
  (`KismetArrayLibrary.Array_Clear` (`self.ModifiersCopy`)))

(fn `ApplyBonusPoint`
  (params (bonus :type Integer))
  (set `self.Point` (`KismetMathLibrary.Max` (`KismetMathLibrary.FCeil` (* (+ bonus (`self.Point`)) (`self.Multiplier`))))))

(fn `ApplyMalusPoint`
  (params (malus :type Integer))
  (set `self.Point` (`KismetMathLibrary.Max` (- (`self.Point`) malus)))
  (set `self.Multiplier` 1.0))

(fn `Boost Multiplier`
  (params (`bonus mult` :type "Float (double-precision)"))
  (set `self.Multiplier` (* (+ `bonus mult` 1.0) (`self.Multiplier`))))

(fn `RemoveAllOppositeTags`
  (params (container :type "Array of /Game/SLICE/BP_Modifier Object Reference (by ref)") (tagsToRemove :type "GameplayTagContainer Structure"))
  (locals (Slice_Bonus_Opposite :type "GameplayTagContainer Structure"))
  (for _array_element container
    (if (`BlueprintGameplayTagLibrary.HasAnyTags` (`/Game/SLICE/BP_Modifier.Slice Tag Container` _array_element) tagsToRemove true)
      (`KismetArrayLibrary.Array_RemoveItem` container _array_element))))

(fn `UserConstructionScript`)